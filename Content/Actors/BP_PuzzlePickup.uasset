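; BP_PuzzlePickup is a puzzle pickup actor with a sprite that the player collects by touching it.
; On box overlap, it checks that the other actor is the BP_PlayerCharacter found in the level, calls Collected with its ID and hides itself.
; It is only hidden, with collision left unchanged, and is shown again on BeginPlay.
; GetSprite exposes the render component's sprite to other code.
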(event `self.ReceiveBeginPlay`
  (`self.SetActorHiddenInGame` false))

(event `self.Box.OnComponentBeginOverlap`
  (params (OverlappedComponent :type "PrimitiveComponent Object Reference") (OtherActor :type "Actor Object Reference") (OtherComp :type "PrimitiveComponent Object Reference") (OtherBodyIndex :type Integer) (bFromSweep :type Boolean) (SweepResult :type "HitResult Structure (by ref)"))
  (bind _returnvalue (`GameplayStatics.GetActorOfClass` "/Game/Actors/BP_PlayerCharacter.BP_PlayerCharacter_C"))
  (if (== _returnvalue OtherActor)
    (`self.Collected` (`self.ID`))
    (`self.SetActorHiddenInGame` true)))

(fn `GetSprite`
  (returns (Sprite :type "PaperSprite Object Reference"))
  (return (`PaperSpriteComponent.GetSprite` (`self.RenderComponent`))))

(fn `UserConstructionScript`)